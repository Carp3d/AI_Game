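; Level 3 access key pickup that the BigBoi_Char player collects.
; It spins around its yaw axis every tick at a constant rate scaled by delta time.
; Overlapping its sphere with BigBoi_Char increments that character's key count, destroys the pickup and prints the new total.
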(event `self.ReceiveTick`
  (params (DeltaSeconds :type "Float (single-precision)"))
  (`self.K2_AddActorLocalRotation` (`KismetMathLibrary.MakeRotator` 0.0 0.0 (* DeltaSeconds 50.0))))

(event `self.Sphere.OnComponentBeginOverlap`
  (params (OverlappedComponent :type "PrimitiveComponent Object Reference") (OtherActor :type "Actor Object Reference") (OtherComp :type "PrimitiveComponent Object Reference") (OtherBodyIndex :type Integer) (bFromSweep :type Boolean) (SweepResult :type "HitResult Structure (by ref)"))
  (bind _asbig_boi_char (cast `/Game/ThirdPersonBP/Blueprints/Characters/BigBoi/BigBoi_Char` OtherActor))
  (bind _output_get (set `/Game/ThirdPersonBP/Blueprints/Characters/BigBoi/BigBoi_Char.NumberofKeys` (+ (`/Game/ThirdPersonBP/Blueprints/Characters/BigBoi/BigBoi_Char.NumberofKeys` _asbig_boi_char) 1) _asbig_boi_char))
  (`self.K2_DestroyActor`)
  (`KismetSystemLibrary.PrintString` (`KismetStringLibrary.Conv_IntToString` _output_get)))

(fn `UserConstructionScript`)