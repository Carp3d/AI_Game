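; LIGHT3 is a flickering light actor that randomly switches between a lit and an unlit state.
; On BeginPlay it hides StaticMesh1, which is shown only in the unlit state.
; Each Tick, a random roll weighted by DeltaSeconds triggers a FlipFlop about once per second on average.
; The FlipFlop alternates between showing PointLight with StaticMesh and showing StaticMesh1 alone.
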(event `self.ReceiveBeginPlay`
  (`SceneComponent.SetVisibility` (`self.StaticMesh1`) false false))

(event `self.ReceiveTick`
  (params (DeltaSeconds :type "Float (single-precision)"))
  (if (>= (+ DeltaSeconds (`KismetMathLibrary.RandomFloat`)) 1.0)
    (`/Engine/EditorBlueprintResources/StandardMacros.FlipFlop`
      (:`A`
        (`SceneComponent.SetVisibility` (`self.PointLight`) true false)
        (`SceneComponent.SetVisibility` (`self.StaticMesh`) true false)
        (`SceneComponent.SetVisibility` (`self.StaticMesh1`) false false))
      (:`B`
        (`SceneComponent.SetVisibility` (`self.PointLight`) false false)
        (`SceneComponent.SetVisibility` (`self.StaticMesh`) false false)
        (`SceneComponent.SetVisibility` (`self.StaticMesh1`) true false)))))

(fn `UserConstructionScript`)